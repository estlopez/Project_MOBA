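; Base turret pawn, paired with a Turret_AI controller, that tracks and fires on a target and can be clicked to be attacked by the player.
; While a target is in range, Tick smoothly rotates the laser mesh toward it.
; ShootEvent starts or clears a looping timer that spawns projectiles at the barrel, based on CanShoot.
; Clicking sets it as the player's target and triggers an attack if close enough.
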(event `self.ReceiveActorOnClicked`
  (params (ButtonPressed :type "Key Structure"))
  (bind _playerref (`self.PlayerRef`))
  (if (== (`GameplayStatics.GetPlayerPawn` 0) _playerref)
    (set `/Game/Blueprints/PlayerBlueprints/BP_TopDownCharacter.CurrentTarget` self _playerref)
    (bind _distance (`/Game/Blueprints/PlayerBlueprints/BP_TopDownCharacter.TargetDistance` _playerref))
    (if (<= _distance 400.0)
      (`/Game/Blueprints/PlayerBlueprints/BP_TopDownCharacter.Attack` _playerref))))

(event `self.ReceiveTick`
  (params (DeltaSeconds :type "Float (single-precision)"))
  (if (`self.TargetInRange?`)
    (`self.LookAtTarget`)))

(event `self.ReceiveBeginPlay`
  (bind _returnvalue (`GameplayStatics.GetActorOfClass` "/Game/Blueprints/PlayerBlueprints/BP_TopDownCharacter.BP_TopDownCharacter_C"))
  (set `self.PlayerRef` _returnvalue)
  (set `self.ControllerRef` (cast `/Game/AutoTurretAsset/TurretAssetFiles/AI_PerceptionFiles/Turret_AI` (`self.GetController`) :!pure true)))

(event `ShootEvent`
  (if (`self.CanShoot?`)
    (bind _returnvalue (`KismetSystemLibrary.K2_SetTimer` null "ProjectileSpawn" (`self.FireInterval - Between Shots`) true))
    (set `self.ProjectileSpawnHandle` _returnvalue)
    (else
      (`KismetSystemLibrary.K2_ClearAndInvalidateTimerHandle` (`self.ProjectileSpawnHandle`)))))

(event `self.ReceiveActorBeginOverlap`
  (params (OtherActor :type "Actor Object Reference")))

(fn `LookAtTarget`
  (bind _lasermesh (`self.LaserMesh`))
  (`/Engine/EditorBlueprintResources/StandardMacros.IsValid` (`self.CurrentTarget`)
    (:`Is Valid`
      (`SceneComponent.K2_SetWorldRotation` _lasermesh (`KismetMathLibrary.RInterpTo` (`SceneComponent.K2_GetComponentRotation` _lasermesh) (`KismetMathLibrary.FindLookAtRotation` (`KismetMathLibrary.MakeVector` (.x (`SceneComponent.K2_GetComponentLocation` _lasermesh)) (.y (`SceneComponent.K2_GetComponentLocation` _lasermesh)) (+ (.z (`SceneComponent.K2_GetComponentLocation` _lasermesh)) 150.0)) (`self.K2_GetActorLocation` (`self.CurrentTarget`))) (`GameplayStatics.GetWorldDeltaSeconds`) (`self.LookAtSpeed`)) false false))))

(fn `ProjectileSpawn`
  (`|SpawnActorFromClass` "/Game/AutoTurretAsset/TurretAssetFiles/Blueprints/Projectile.Projectile_C" (`SceneComponent.K2_GetComponentToWorld` (`self.Barrel`)) "Undefined" "OverrideRootScale" null self))

(fn `UserConstructionScript`)