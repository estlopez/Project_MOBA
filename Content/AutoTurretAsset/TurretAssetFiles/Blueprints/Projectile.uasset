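; Projectile actor for the auto turret asset that damages whatever actor its collider overlaps.
; On BeginPlay it casts its instigator to BaseTurret_perception and stores it, and only if that succeeds starts a timer that destroys it after a few seconds.
; An overlap applies fixed damage, prints the hit actor's name on screen, and destroys the projectile immediately.
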(event `self.ReceiveBeginPlay`
  (bind _asbase_turret_perception (cast `/Game/AutoTurretAsset/TurretAssetFiles/Blueprints/BaseTurret_perception` (`self.GetInstigator`)))
  (set `self.As Base Turret Perception` _asbase_turret_perception)
  (`KismetSystemLibrary.K2_SetTimer` null "KillSelf" 5.0))

(event `self.Collider.OnComponentBeginOverlap`
  (params (OverlappedComponent :type "PrimitiveComponent Object Reference") (OtherActor :type "Actor Object Reference") (OtherComp :type "PrimitiveComponent Object Reference") (OtherBodyIndex :type Integer) (bFromSweep :type Boolean) (SweepResult :type "HitResult Structure (by ref)"))
  (`GameplayStatics.ApplyDamage` OtherActor 50.0)
  (`KismetSystemLibrary.PrintString` (`KismetSystemLibrary.GetDisplayName` OtherActor) true false (struct :`R` 1.0 :`G` 0.050213 :`A` 1.0))
  (`self.KillSelf`))

(fn `KillSelf`
  (`self.K2_DestroyActor`))

(fn `UserConstructionScript`)