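; BPC_Attack is an attack component whose LineTrace function finds and validates a target between a clicked location and the input actor.
; It capsule-traces from the click to that actor against WorldDynamic objects, ignoring the actor and its weapon, with timed debug drawing.
; The hit actor becomes CurrentTarget, which is valid if it reports being targetable and implements BPI_TeamIndentifiable.
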(fn `LineTrace`
  (params (InputClass :type "Actor Object Reference") (ClickLocation :type "Vector Structure"))
  (returns (ValidTarget :type Boolean))
  (bind _outhit (`KismetSystemLibrary.CapsuleTraceSingleForObjects` ClickLocation (`Actor.K2_GetActorLocation` InputClass) 50.0 75.0 (`|MakeArray` "ObjectTypeQuery2" :!type "EObjectTypeQuery Enum") false (`|MakeArray` InputClass (`self.WeaponRef`) :!type "Actor Object Reference") "ForDuration"))
  (bind _output_get (set `self.CurrentTarget` (`.HitActor` (`GameplayStatics.BreakHitResult` _outhit))))
  (`/Engine/EditorBlueprintResources/StandardMacros.IsValid` _output_get
    (:`Is Valid`
      (bind _isalive_ (message `/Game/Blueprints/BPI_TeamIndentifiable.CanBeTargeted` _output_get))
      (bind _output_get_2 (set `self.ValidTarget` (and _isalive_ (`KismetSystemLibrary.DoesImplementInterface` _output_get "/Game/Blueprints/BPI_TeamIndentifiable.BPI_TeamIndentifiable_C"))))
      (return _output_get_2))))