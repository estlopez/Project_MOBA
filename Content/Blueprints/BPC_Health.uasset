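; Health component that tracks current health for its owning actor and handles death.
; CurrentHealth starts at MaxHealth on BeginPlay, and TakeDamage subtracts damage, calling Die at zero or below.
; Die sets IsDead, fires OnDeath and plays a 2D white noise sound at a very low randomized pitch.
; TakeDamage does not check IsDead, so further hits after death run Die again.
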(event `self.ReceiveBeginPlay`
  (set `self.CurrentHealth` (`self.MaxHealth`)))

(fn `Die`
  (set `self.bIsDead` true)
  (`self.OnDeath`)
  (`GameplayStatics.PlaySound2D` "/Engine/EngineSounds/WhiteNoise.WhiteNoise" 0.5 (`KismetMathLibrary.RandomFloatInRange` 0.01 0.05) 0.3 null null))

(fn `TakeDamage`
  (params (DamageAmount :type "Float (double-precision)"))
  (bind _output_get (set `self.CurrentHealth` (- (`self.CurrentHealth`) DamageAmount)))
  (if (<= _output_get 0.0)
    (`self.Die`)))