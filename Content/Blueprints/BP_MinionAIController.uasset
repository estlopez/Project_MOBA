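; AI controller for minions that halts or resumes the controlled pawn's movement as it perceives actors on another team.
; On perception updates, it compares team IDs through interface messages and stores each differing actor as CurrentTarget, so the last match wins.
; It stops the pawn if that target can be targeted, otherwise starts it moving.
; A binding to each target's OnDestroyed event also restarts movement.
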(event `self.AIPerception.OnPerceptionUpdated`
  (params (UpdatedActors :type "Array of Actor Object Reference (by ref)"))
  (bind _returnvalue (`self.K2_GetPawn`))
  (for _array_element UpdatedActors
    (`/Engine/EditorBlueprintResources/StandardMacros.IsValid` _array_element
      (:`Is Valid`
        (if (`KismetSystemLibrary.DoesImplementInterface` _array_element "/Game/Blueprints/BPI_TeamIndentifiable.BPI_TeamIndentifiable_C")
          (bind _eteam (message `/Game/Blueprints/BPI_TeamIndentifiable.GetTeamID` _array_element))
          (bind _eteam_2 (message `/Game/Blueprints/BPI_TeamIndentifiable.GetTeamID` _returnvalue))
          (if (`|EnumInequality` _eteam _eteam_2)
            (bind _output_get (set `self.CurrentTarget` _array_element))
            (add `self.OnDestroyed` _output_get (delegate `OnDestroyed_Event`))
            (bind _isalive_ (message `/Game/Blueprints/BPI_TeamIndentifiable.CanBeTargeted` _output_get))
            (if _isalive_
              (message `/Game/Blueprints/BPI_Attack.StopMoving` _returnvalue)
              (else
                (message `/Game/Blueprints/BPI_Attack.StartMoving` _returnvalue)))))))))

(event `OnDestroyed_Event` :!signature `self.OnDestroyed`
  (params (DestroyedActor :type "Actor Object Reference"))
  (message `/Game/Blueprints/BPI_Attack.StartMoving` (`self.K2_GetPawn`)))

(fn `UserConstructionScript`)