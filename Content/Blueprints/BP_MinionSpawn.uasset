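; BP_MinionSpawn is a lane spawner that continuously spawns BP_Minion actors at its own transform.
; On BeginPlay it copies its LaneSelectors value into the LaneTarget's LaneNumber, then starts a looping two-second timer calling SpawnMinion.
; Each new minion receives the lane number and LaneTarget reference, then is appended to CreepArray.
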(event `self.ReceiveBeginPlay`
  (`self.SetLaneTarget`)
  (`KismetSystemLibrary.K2_SetTimer` null "SpawnMinion" 2.0 true))

(fn `SetLaneTarget`
  (set `/Game/Blueprints/BP_Lane.LaneNumber` (`self.LaneSelectors`) (`self.LaneTarget`)))

(fn `SpawnMinion`
  (bind _returnvalue (`|SpawnActorFromClass` "/Game/Blueprints/BP_Minion.BP_Minion_C" (`self.GetTransform`) "Undefined" "MultiplyWithRoot" null null))
  (bind _output_get (set `self.CurrentSpawn` _returnvalue))
  (set `/Game/Blueprints/BP_Minion.LaneNumber` (`self.LaneSelectors`) _output_get)
  (set `/Game/Blueprints/BP_Minion.LaneTarget` (`self.LaneTarget`) _output_get)
  (`KismetArrayLibrary.Array_Add` (`self.CreepArray`) _output_get))

(fn `UserConstructionScript`)