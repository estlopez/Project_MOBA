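; Short-lived slash attack hitbox that damages actors on a different team from its instigator.
; When its collider overlaps an actor, it compares that actor's team ID with the instigator's and applies its damage value if they differ.
; It destroys itself after a brief delay from spawn, with a hit also leading into a delayed destroy.
; It reports its own team ID and marks itself as untargetable.
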(event `self.ReceiveBeginPlay`
  (`KismetSystemLibrary.Delay` 0.2)
  (`self.K2_DestroyActor` self :!label _label))

(event `self.Collider.OnComponentBeginOverlap`
  (params (OverlappedComponent :type "PrimitiveComponent Object Reference") (OtherActor :type "Actor Object Reference") (OtherComp :type "PrimitiveComponent Object Reference") (OtherBodyIndex :type Integer) (bFromSweep :type Boolean) (SweepResult :type "HitResult Structure (by ref)"))
  (bind _returnvalue (`self.GetInstigator`))
  (`/Engine/EditorBlueprintResources/StandardMacros.IsValid` OtherActor
    (:`Is Valid`
      (bind _eteam (message `/Game/Blueprints/BPI_TeamIndentifiable.GetTeamID` OtherActor))
      (`/Engine/EditorBlueprintResources/StandardMacros.IsValid` _returnvalue
        (:`Is Valid`
          (bind _eteam_2 (message `/Game/Blueprints/BPI_TeamIndentifiable.GetTeamID` _returnvalue))
          (if (`|EnumInequality` _eteam_2 _eteam)
            (`GameplayStatics.ApplyDamage` OtherActor (`self.DamageValue`))
            (`KismetSystemLibrary.Delay` 0.2)
            (goto _label)))))))

(fn `CanBeTargeted`
  (returns (`isAlive?` :type Boolean))
  (return false))

(fn `GetTeamID`
  (returns (ETeam :type "/Game/Blueprints/ENum_TeamID Enum"))
  (return (`self.TeamID`)))

(fn `UserConstructionScript`)