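; BP_EnemyHero is an AI-controlled enemy hero character that spawns a weapon on its hand socket and attacks via montage.
; Team ID, alive state and target distance functions support targeting, while Die clears the AI_EnemyHero blackboard target.
; AnyDamage sets health to damage minus current health (reversed subtraction), destroying hero and weapon at zero or below without calling Die.
; Respawn restores visibility, start transform and health, then re-enables targeting after a short timer.
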(event `/Game/Blueprints/BPI_Attack.DoAttack`
  (`self.Attack`))

(event `self.ReceiveBeginPlay`
  (bind _returnvalue (`|SpawnActorFromClass` "/Game/Blueprints/PlayerBlueprints/BP_Weapon.BP_Weapon_C" (`SceneComponent.GetSocketTransform` (`self.Mesh`) "hand_rSocket" "RTS_World") "Undefined" "MultiplyWithRoot" null null))
  (set `self.SpawnedWeapon` _returnvalue)
  (`SceneComponent.K2_AttachToComponent` (`Actor.RootComponent` _returnvalue) (`self.Mesh`) "hand_rSocket" "SnapToTarget" "SnapToTarget" "KeepRelative" true)
  (set `self.isAlive?` true)
  (set `self.StartingLocation` (`self.GetTransform`)))

(event `self.ReceiveAnyDamage`
  (params (Damage :type "Float (single-precision)") (DamageType :type "DamageType Object Reference") (InstigatedBy :type "Controller Object Reference") (DamageCauser :type "Actor Object Reference"))
  (bind _bpc_health (`self.BPC_Health`))
  (if (`ActorComponent.ComponentHasTag` (`self.BPC_Health`) "BPC_Health")
    (bind _output_get (set `/Game/Blueprints/BPC_Health.CurrentHealth` (- Damage (`/Game/Blueprints/BPC_Health.CurrentHealth` _bpc_health)) _bpc_health))
    (if (<= _output_get 0.0)
      (`KismetSystemLibrary.PrintString` (`KismetStringLibrary.Conv_DoubleToString` _output_get) true false (struct :`G` 1.0 :`B` 0.093859 :`A` 1.0))
      (`self.K2_DestroyActor`)
      (`self.K2_DestroyActor` (`self.SpawnedWeapon`)))))

(fn `Attack`
  (`self.PlayAnimMontage` "/Game/AutoTurretAsset/ExampleContent/Characters/Mannequins/Animations/MON_Attack.MON_Attack"))

(fn `CanBeTargeted`
  (returns (`isAlive?` :type Boolean))
  (return (`self.isAlive?`)))

(fn `Die`
  (set `self.isAlive?` false)
  (bind _asai_enemy_hero (cast `/Game/Blueprints/PlayerBlueprints/AI_EnemyHeroFolder/AI_EnemyHero` (`self.GetController`)))
  (`BlackboardComponent.ClearValue` (`AIController.Blackboard` _asai_enemy_hero) (`self.TargetActor`)))

(fn `GetTeamID`
  (returns (ETeam :type "/Game/Blueprints/ENum_TeamID Enum"))
  (return (`self.TeamID`)))

(fn `Respawn`
  (`SceneComponent.SetVisibility` (`self.Mesh`) true true)
  (`self.K2_SetActorTransform` (`self.StartingLocation`))
  (set `/Game/Blueprints/BPC_Health.CurrentHealth` 1000.0 (`self.BPC_Health`))
  (`KismetSystemLibrary.K2_SetTimer` null "SetLive" 0.5))

(fn `SetLive`
  (set `self.isAlive?` true))

(fn `TargetDistance`
  (returns (Distance :type "Float (double-precision)"))
  (bind _output_get (set `self.DistanceToTarget` (`self.GetDistanceTo` (`self.CurrentTarget`))))
  (return _output_get))

(fn `UserConstructionScript`)